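; BP_Enemy is a spinning cube enemy that damages the player or awards points when it is hit.
; Tick rotates the Cube on all three axes at EnemyRotationSpeed.
; A custom overlap-style event casts to BP_Player: on success it shakes the camera, applies damage, plays HUD feedback, self-destructs and shows restart upon death.
; Any other actor destroys the enemy and adds EnemyPoints to the player's score.
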(event `self.ReceiveTick`
  (params (DeltaSeconds :type "Float (single-precision)"))
  (bind _returnvalue (* DeltaSeconds (`self.Enemy_RotationSpeed`)))
  (`SceneComponent.K2_AddWorldRotation` (`self.Cube`) (`KismetMathLibrary.MakeRotator` _returnvalue _returnvalue _returnvalue) false false))

(event `CustomEvent`
  (params (OverlappedComponent :type "PrimitiveComponent Object Reference") (OtherActor :type "Actor Object Reference") (OtherComp :type "PrimitiveComponent Object Reference") (OtherBodyIndex :type Integer) (bFromSweep :type Boolean) (SweepResult :type "HitResult Structure (by ref)"))
  (bind _asbp_player (cast `/Game/InfiniteMatrix/Blueprints/BP_Player` OtherActor)
    (:`then`
      (`GameplayStatics.PlayWorldCameraShake` "/Game/InfiniteMatrix/Blueprints/BP_Camera_Shake.BP_Camera_Shake_C" (`self.K2_GetActorLocation` _asbp_player) 0.0 1000.0)
      (`/Game/InfiniteMatrix/Blueprints/BP_Player.Update Health` _asbp_player (`self.Enemy_Dmg`))
      (`/Game/InfiniteMatrix/UI/Game_Hub.PlayDamageAnimate` (`/Game/InfiniteMatrix/Blueprints/BP_Player.GameHubWidget` _asbp_player))
      (`self.K2_DestroyActor`)
      (if (`/Game/InfiniteMatrix/Blueprints/BP_Player.IsDead` _asbp_player)
        (`/Game/InfiniteMatrix/Blueprints/BP_Player.DisplayRestart` _asbp_player)))
    (:`CastFailed`
      (`self.K2_DestroyActor`)
      (bind _returnvalue (`GameplayStatics.GetActorOfClass` "/Game/InfiniteMatrix/Blueprints/BP_Player.BP_Player_C"))
      (`/Game/InfiniteMatrix/Blueprints/BP_Player.UpdateScore` _returnvalue (`self.Enemy_Points`) false))))

(event `self.Cube.OnComponentBeginOverlap`
  (params (OverlappedComponent :type "PrimitiveComponent Object Reference") (OtherActor :type "Actor Object Reference") (OtherComp :type "PrimitiveComponent Object Reference") (OtherBodyIndex :type Integer) (bFromSweep :type Boolean) (SweepResult :type "HitResult Structure (by ref)"))
  ;[1 1 1] old
)

(fn `UserConstructionScript`)