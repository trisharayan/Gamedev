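; BP_Projectile is a projectile that accounts for the player ship's motion and removes itself on overlap.
; A custom event adds the BP_Player's forward speed to the ProjectileMovement initial and maximum speeds.
; An overlap handler ignores the player, starts a short lifespan on a BP_Tunnel trigger zone, and destroys the projectile on any other contact.
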(event `CustomEvent`
  (bind _projectilemovement (`self.ProjectileMovement`))
  (bind _asbp_player (cast `/Game/InfiniteMatrix/Blueprints/BP_Player` (`GameplayStatics.GetPlayerPawn` 0)))
  (bind _forwardspeed (`/Game/InfiniteMatrix/Blueprints/BP_Player.ForwardSpeed` _asbp_player))
  (set `ProjectileMovementComponent.InitialSpeed` (+ 6000.0 _forwardspeed) _projectilemovement)
  (set `ProjectileMovementComponent.MaxSpeed` (+ 10000.0 _forwardspeed) _projectilemovement))

(event `CustomEvent_1`
  (params (OverlappedComponent :type "PrimitiveComponent Object Reference") (OtherActor :type "Actor Object Reference") (OtherComp :type "PrimitiveComponent Object Reference") (OtherBodyIndex :type Integer) (bFromSweep :type Boolean) (SweepResult :type "HitResult Structure (by ref)"))
  (bind _asbp_tunnel (cast `/Game/InfiniteMatrix/Blueprints/BP_Tunnel` OtherActor)
    (:`then`
      (if (== (`/Game/InfiniteMatrix/Blueprints/BP_Tunnel.TriggerZone` _asbp_tunnel) OtherComp)
        (`self.SetLifeSpan` 2.0)
        (else
          (`self.K2_DestroyActor`))))
    (:`CastFailed`
      (if (not (`KismetMathLibrary.ClassIsChildOf` (`GameplayStatics.GetObjectClass` OtherActor) "/Game/InfiniteMatrix/Blueprints/BP_Player.BP_Player_C"))
        (`self.K2_DestroyActor`)))))

(fn `UserConstructionScript`)