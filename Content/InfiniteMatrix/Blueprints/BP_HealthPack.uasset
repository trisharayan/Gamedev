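; BP_HealthPack is a single-use health pickup that adjusts the player's health on overlap.
; When BP_Player overlaps TriggerBox, it passes a random integer, bounded by truncated HealthValue and a fixed maximum, to UpdateHealth.
; It then adds a HitScreen1 widget to the viewport and destroys itself.
; A custom event with an overlap signature duplicates this logic, with no binding or call in the graph.
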(event `CustomEvent`
  (params (OverlappedComponent :type "PrimitiveComponent Object Reference") (OtherActor :type "Actor Object Reference") (OtherComp :type "PrimitiveComponent Object Reference") (OtherBodyIndex :type Integer) (bFromSweep :type Boolean) (SweepResult :type "HitResult Structure (by ref)"))
  (bind _asbp_player (cast `/Game/InfiniteMatrix/Blueprints/BP_Player` OtherActor))
  (`/Game/InfiniteMatrix/Blueprints/BP_Player.Update Health` _asbp_player (`KismetMathLibrary.Conv_IntToDouble` (`KismetMathLibrary.RandomIntegerInRange` (`KismetMathLibrary.FTrunc` (`self.HealthValue`)) 20)))
  (bind _returnvalue (`|CreateWidget` "/Game/InfiniteMatrix/UI/HitScreen1.HitScreen1_C"))
  (`UserWidget.AddToViewport` _returnvalue 0)
  (`self.K2_DestroyActor`))

(event `self.TriggerBox.OnComponentBeginOverlap`
  (params (OverlappedComponent :type "PrimitiveComponent Object Reference") (OtherActor :type "Actor Object Reference") (OtherComp :type "PrimitiveComponent Object Reference") (OtherBodyIndex :type Integer) (bFromSweep :type Boolean) (SweepResult :type "HitResult Structure (by ref)"))
  (bind _asbp_player (cast `/Game/InfiniteMatrix/Blueprints/BP_Player` OtherActor))
  (`/Game/InfiniteMatrix/Blueprints/BP_Player.Update Health` _asbp_player (`KismetMathLibrary.Conv_IntToDouble` (`KismetMathLibrary.RandomIntegerInRange` (`KismetMathLibrary.FTrunc` (`self.HealthValue`)) 20)))
  (bind _returnvalue (`|CreateWidget` "/Game/InfiniteMatrix/UI/HitScreen1.HitScreen1_C"))
  (`UserWidget.AddToViewport` _returnvalue 0)
  (`self.K2_DestroyActor`))

(fn `UserConstructionScript`)