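; BP_Tunnel is one segment of an endless tunnel, with a spinning holed wall the player must pass through.
; Functions randomize the wall mesh and roll, spawn an enemy, and roll a chance for a health pack.
; Hitting the wall damages the player, shows hit feedback and offers restart on death.
; A trigger behind the wall updates score or life loss, requests the next segment, then destroys this one and its spawned actors.
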(event `self.ReceiveTick`
  (params (DeltaSeconds :type "Float (single-precision)"))
  (`SceneComponent.K2_AddLocalRotation` (`self.WallMesh`) (`KismetMathLibrary.MakeRotator` (* DeltaSeconds (`self.RotateSpeed`))) false false))

(event `self.TriggerZone.OnComponentBeginOverlap`
  (params (OverlappedComponent :type "PrimitiveComponent Object Reference") (OtherActor :type "Actor Object Reference") (OtherComp :type "PrimitiveComponent Object Reference") (OtherBodyIndex :type Integer) (bFromSweep :type Boolean) (SweepResult :type "HitResult Structure (by ref)"))
  (bind _healthpack (`self.HealthPack`))
  (bind _enemyref (`self.EnemyRef`))
  (bind _asbp_player (cast `/Game/InfiniteMatrix/Blueprints/BP_Player` OtherActor))
  (`/Game/InfiniteMatrix/Blueprints/BP_Player.UpdateScore` _asbp_player (`self.HolePoints`) (`self.isWallHit`)) ; Only update score if wall is not hit
  (set `self.isWallHit` false) ; The trigger zone is behind the wall, so we can\nreset isWallHit flag once the player passes\nthe trigger zone.
  (`/Game/InfiniteMatrix/Blueprints/BP_TunnelSpawner.SpawnTunnelAtSpawnPoint` (`self.TunnelSpawner`))
  (`self.K2_DestroyActor`)
  (`/Engine/EditorBlueprintResources/StandardMacros.IsValid` _enemyref
    (:`Is Valid`
      (`self.K2_DestroyActor` _enemyref))
    (:`Is Not Valid`
      _))
  (`/Engine/EditorBlueprintResources/StandardMacros.IsValid` _healthpack ; see if health pack appears in the current tunnel
    (:`Is Valid`
      (`self.K2_DestroyActor` _healthpack))))

(event `self.WallMesh.OnComponentBeginOverlap`
  (params (OverlappedComponent :type "PrimitiveComponent Object Reference") (OtherActor :type "Actor Object Reference") (OtherComp :type "PrimitiveComponent Object Reference") (OtherBodyIndex :type Integer) (bFromSweep :type Boolean) (SweepResult :type "HitResult Structure (by ref)"))
  (set `self.isWallHit` (`KismetMathLibrary.ClassIsChildOf` (`GameplayStatics.GetObjectClass` OtherActor) "/Game/InfiniteMatrix/Blueprints/BP_Player.BP_Player_C")) ; player hit the wall ?
  (bind _asbp_player (cast `/Game/InfiniteMatrix/Blueprints/BP_Player` OtherActor))
  (bind _returnvalue (`|CreateWidget` "/Game/InfiniteMatrix/UI/HitScreen.HitScreen_C"))
  (`UserWidget.AddToViewport` _returnvalue 0)
  (`/Game/InfiniteMatrix/Blueprints/BP_Player.Update Health` _asbp_player (`self.Damage`)) ; udpate health before checking dead
  (`/Game/InfiniteMatrix/UI/Game_Hub.PlayDamageAnimate` (`/Game/InfiniteMatrix/Blueprints/BP_Player.GameHubWidget` _asbp_player))
  (if (`/Game/InfiniteMatrix/Blueprints/BP_Player.IsDead` _asbp_player)
    (`/Game/InfiniteMatrix/Blueprints/BP_Player.DisplayRestart` _asbp_player)))

(event `CustomEvent`
  (params (OverlappedComponent :type "PrimitiveComponent Object Reference") (OtherActor :type "Actor Object Reference") (OtherComp :type "PrimitiveComponent Object Reference") (OtherBodyIndex :type Integer) (bFromSweep :type Boolean) (SweepResult :type "HitResult Structure (by ref)"))
  ;[1 1 1] Here
)

(fn `GenerateEnemy`
  (bind _returnvalue_location (`KismetMathLibrary.BreakTransform` (`self.GetTransform`)))
  (bind _returnvalue (`|SpawnActorFromClass` "/Game/InfiniteMatrix/Blueprints/BP_Enemy.BP_Enemy_C" (`KismetMathLibrary.MakeTransform` (+ _returnvalue_location (`KismetMathLibrary.MakeVector` (`KismetMathLibrary.Conv_IntToDouble` (`KismetMathLibrary.RandomIntegerInRange` 1500 2300)) (`KismetMathLibrary.Conv_IntToDouble` (`KismetMathLibrary.RandomIntegerInRange` -275 275)) (`KismetMathLibrary.Conv_IntToDouble` (`KismetMathLibrary.RandomIntegerInRange` -275 275))))) "Undefined" "MultiplyWithRoot" null null))
  (set `self.EnemyRef` _returnvalue))

(fn `GenerateHealthPack`
  (bind (_returnvalue_x _returnvalue_y _returnvalue_z) (`KismetMathLibrary.BreakVector` (`self.K2_GetActorLocation`)))
  (if (< (`KismetMathLibrary.RandomInteger` 100) (`self.PackProb`))
    (bind _returnvalue (`|SpawnActorFromClass` "/Game/InfiniteMatrix/Blueprints/BP_HealthPack.BP_HealthPack_C" (`KismetMathLibrary.MakeTransform` (`KismetMathLibrary.MakeVector` (+ (`KismetMathLibrary.RandomIntegerInRange` 7000 300) _returnvalue_x) (+ _returnvalue_y (`KismetMathLibrary.RandomIntegerInRange` 0 300)) (+ _returnvalue_z (`KismetMathLibrary.RandomIntegerInRange` 0 300)))) "Undefined" "MultiplyWithRoot" null null))
    (set `self.HealthPack` _returnvalue)))

(fn `RandomizeWall`
  (`StaticMeshComponent.SetStaticMesh` (`self.WallMesh`) (select `int` (`KismetMathLibrary.RandomIntegerInRange` 0 3) :`0` "/Game/InfiniteMatrix/Meshes/SM_Hole_01.SM_Hole_01" :`1` "/Game/InfiniteMatrix/Meshes/SM_Hole_02.SM_Hole_02" :`2` "/Game/InfiniteMatrix/Meshes/SM_Hole_03.SM_Hole_03" :`3` "/Game/InfiniteMatrix/Meshes/SM_Hole_04.SM_Hole_04" :!type "StaticMesh Object Reference"))
  (`SceneComponent.K2_AddLocalRotation` (`self.WallMesh`) (`KismetMathLibrary.MakeRotator` (`KismetMathLibrary.RandomFloatInRange` 0.0 360.0)) false false))

(fn `UserConstructionScript`)